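; Player fighter character for a 2D fighting game, handling side movement, jump, crouch, attack input and health.
; Inputs are recorded in an array cleared by a timer started on attack presses; heavy attack is only recorded.
; Sphere hurt boxes snap to mesh sockets by matching component names to map keys.
; Activating the left-hand box checks overlaps for another actor's skeletal mesh, then sends damage through an interface to its health component.
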(event `self.ReceiveBeginPlay`
  (`/Game/_Main/Functions/L_CharacterMacros.Set Input Mapping Context` "/Game/_Main/Input/IAC_FightingInput2D.IAC_FightingInput2D" (`self.Index`)
    (:`Exec`
      (`self.F_RegisterHurtBoxes`))))

(event `EnhancedInput|/Game/_Main/Input/IA_MoveRight`
  (params (ActionValue :type "Float (single-precision)") (ElapsedSeconds :type "Float (single-precision)") (TriggeredSeconds :type "Float (single-precision)"))
  (:`Triggered`
    (`self.F_MoveRight` ActionValue)))

(event `EnhancedInput|/Game/_Main/Input/IA_JumpCrouch`
  (params (ActionValue :type "Float (single-precision)") (ElapsedSeconds :type "Float (single-precision)") (TriggeredSeconds :type "Float (single-precision)"))
  (:`Triggered`
    (`self.F_JumpCrouch` ActionValue))
  (:`Completed`
    (`self.F_ResetCrouch`)))

(event `self.OnLanded`
  (params (Hit :type "HitResult Structure (by ref)"))
  (set `self.IsJumping` false))

(event `EnhancedInput|/Game/_Main/Input/IA_LightAttack`
  (params (ActionValue :type Boolean) (ElapsedSeconds :type "Float (single-precision)") (TriggeredSeconds :type "Float (single-precision)"))
  (:`Triggered`
    (if (not (`self.LightAttack`))
      (`self.F_TrackInput` "NewEnumerator0" true)
      (set `self.LightAttack` true))))

(event `Event Reset Light Attack`
  (set `self.LightAttack` false))

(event `Event Activate Light Attack Hurt Box`
  (`ActorComponent.Activate` (`self.LeftHand`) false))

(event `Event Deactivate Light Attack Hurt Box`
  (`ActorComponent.Deactivate` (`self.LeftHand`)))

(event `self.LeftHand.OnComponentActivated`
  (params (Component :type "ActorComponent Object Reference") (bReset :type Boolean))
  (`self.F_TryDealDamage` Component 5.0))

(event `EnhancedInput|/Game/_Main/Input/IA_HeavyAttack`
  (params (ActionValue :type Boolean) (ElapsedSeconds :type "Float (single-precision)") (TriggeredSeconds :type "Float (single-precision)"))
  (:`Triggered`
    (`self.F_TrackInput` "NewEnumerator1" true)))

(event `Event On Input End`
  (`KismetSystemLibrary.K2_SetTimerDelegate` (delegate `Event Clear Input Array`) 0.4))

(event `Event Clear Input Array`
  (`/Game/_Main/Functions/L_CharacterMacros.Clear Tracked Input` (`self.LastInputArray`)
    (:`Exec`
      (`KismetSystemLibrary.PrintString` "Input Reset" true true (struct :`G` 0.66 :`B` 1.0 :`A` 1.0) 0.2))))

(event `Event Receive Damage`
  (params (Amount :type "Float (double-precision)"))
  (bind _health (`/Game/_Main/Components/AC_HealthComponent.F_ModifyHealth` (`self.AC_HealthComponent`) true Amount))
  (`KismetSystemLibrary.PrintString` (`KismetStringLibrary.Conv_DoubleToString` _health)))

(fn `F_Crouch`
  (returns (Continue :type Boolean))
  (if (`self.IsJumping`)
    _
    (elif (`self.IsCrouching`)
      _
      (else
        (`self.Crouch`)
        (bind _output_get (set `self.IsCrouching` true))
        (return _output_get))))
  (return false))

(fn `F_DirectHurtBoxToSocket`
  (params (`Hurt Box` :type "SphereComponent Object Reference"))
  (bind _keys (`BlueprintMapLibrary.Map_Keys` (`self.HurtBoxMap`)))
  (for _array_element _keys
    (if (`KismetStringLibrary.Contains` (`KismetSystemLibrary.GetDisplayName` `Hurt Box`) _array_element)
      (`SceneComponent.K2_AttachToComponent` `Hurt Box` (`self.Mesh`) (`BlueprintMapLibrary.Map_Find` (`self.HurtBoxMap`) _array_element) "SnapToTarget" "SnapToTarget" "KeepRelative" true))))

(fn `F_GetAnimVars`
  (returns (Jumping :type Boolean) (Falling :type Boolean) (Crouching :type Boolean) (Speed :type "Float (double-precision)") (LightAttack :type Boolean))
  (bind _charactermovement (`self.CharacterMovement`))
  (return (`self.IsJumping`) (`NavMovementComponent.IsFalling` _charactermovement) (`self.IsCrouching`) (`KismetMathLibrary.VSize` (`MovementComponent.Velocity` _charactermovement)) (`self.LightAttack`)))

(fn `F_Jump`
  (returns (Continue :type Boolean))
  (if (`self.IsJumping`)
    (return false)
    (else
      (`self.Jump`)
      (bind _output_get (set `self.IsJumping` true))
      (return _output_get))))

(fn `F_JumpCrouch`
  (params (Value :type "Float (double-precision)"))
  (`/Game/_Main/Functions/L_CharacterMacros.Detect Float Direction` Value
    (:`Positive`
      (bind _continue (`self.F_Jump`))
      (`/Game/_Main/Functions/L_LogicMacros.Continue` _continue
        (:`Yes`
          (bind _output_get (set `self.LastJumpCrouchInput` "NewEnumerator4"))
          (`self.F_TrackInput` _output_get))))
    (:`Negative`
      (bind _continue_2 (`self.F_Crouch`))
      (`/Game/_Main/Functions/L_LogicMacros.Continue` _continue_2
        (:`Yes`
          (bind _output_get_2 (set `self.LastJumpCrouchInput` "NewEnumerator5"))
          (`self.F_TrackInput` _output_get_2))))
    (:`Zero`
      (`KismetSystemLibrary.PrintString` "This Should Never Run"))))

(fn `F_MoveRight`
  (params (Value :type "Float (double-precision)"))
  (`self.AddMovementInput` (`self.GetActorRightVector` (`self.GetController`)) Value))

(fn `F_RegisterHurtBoxes`
  (bind _output_get (set `self.HurtBoxes` (`self.K2_GetComponentsByClass` "/Script/Engine.SphereComponent")))
  (for _array_element _output_get
    (`self.F_DirectHurtBoxToSocket` _array_element)))

(fn `F_ResetCrouch`
  (if (`|EnumEquality` (`self.LastJumpCrouchInput`) "NewEnumerator5")
    (`self.UnCrouch`)
    (set `self.IsCrouching` false)))

(fn `F_ResetHitAndPassDamage`
  (params (Damage :type "Float (double-precision)"))
  (bind _fighter2d (message `/Game/_Main/Character/INT_Fighter2D.INT Get Fighter2D` (`ActorComponent.GetOwner` (`self.HitMesh`))))
  (`self.Event Receive Damage` _fighter2d (`local.Damage`))
  (set `self.HitMesh` null))

(fn `F_TrackInput`
  (params (Input :type "/Game/_Main/Functions/E_LastInput Enum" :default "NewEnumerator0") (`Start Input Timer` :type Boolean) (Print :type Boolean))
  (bind _lastinputarray (`self.LastInputArray`))
  (`/Game/_Main/Functions/L_CharacterMacros.Track Input` Input _lastinputarray
    (:`Exec`
      (if `Start Input Timer`
        (`self.Event On Input End`))
      (if Print
        (`/Game/_Main/Functions/L_CharacterMacros.Print Input Array` _lastinputarray)))))

(fn `F_TryDealDamage`
  (params (Component :type "ActorComponent Object Reference") (Damage :type "Float (double-precision)"))
  (`KismetArrayLibrary.Array_Clear` (`self.Overlapping Components`))
  (bind _output_get (set `self.Overlapping Components` (`PrimitiveComponent.GetOverlappingComponents` (cast `SphereComponent` Component :!pure true))))
  (`self.Event Deactivate Light Attack Hurt Box`)
  (`self.M Filter Skeletal Mesh` _output_get
    (:`Valid`
      (`self.F_ResetHitAndPassDamage` (`local.Damage`)))))

(fn `INT Get Fighter2D`
  (returns (Fighter2D :type "/Game/_Main/Character/BP_Fighter2D Object Reference"))
  (return self))

(fn `UserConstructionScript`)