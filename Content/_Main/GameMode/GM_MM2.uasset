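; GM_MM2 is a main menu game mode that handles menu widget creation and menu character spawning.
; A server-named event creates W_MainMenu for player controller 1, then a client-named event adds it to the viewport.
; SpawnPlayer spawns a BP_MainMenuCharacter at an input receiver's transform and has that index's controller possess it.
; BeginPlay and both getters are stubs, and the player-start and input-receiver setup is left disconnected.
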(event `self.ReceiveBeginPlay`)

(event `SERVER Create W_MainMenu`
  (bind _returnvalue (`|CreateWidget` "/Game/_Main/UI/W_MainMenu.W_MainMenu_C" (`GameplayStatics.GetPlayerController` 1)))
  (set `self.W_MainMenu` _returnvalue)
  (`self.CLIENT Show W_MainMenu`))

(event `CLIENT Show W_MainMenu`
  (`UserWidget.AddToViewport` (`self.W_MainMenu`) 0))

(fn `F_GetPlayerStarts`
  (bind _outactors (`GameplayStatics.GetAllActorsOfClass` "/Game/_Main/GameMode/BP_PlayerStart.BP_PlayerStart_C"))
  (set `self.PlayerStartArray` _outactors))

(fn `F_SpawnInputRecievers`
  (locals (Index :type Integer)))

(fn `Get Fighter2D`
  (returns (Fighter2D :type "/Game/_Main/GameMode/GM_Fighter2D Object Reference"))
  (return null))

(fn `Get Main Menu`
  (returns (`Main Menu` :type "/Game/_Main/GameMode/GM_MainMenu Object Reference"))
  (`KismetSystemLibrary.PrintString` "Function Not Set Up")
  (return null))

(fn `PF_ConvertNameToInt`
  (params (`Player Start` :type "PlayerStart Object Reference"))
  (returns (ReturnValue :type Integer))
  (return (`KismetStringLibrary.Conv_StringToInt` (`KismetStringLibrary.Conv_NameToString` (`PlayerStart.PlayerStartTag` `Player Start`)))))

(fn `Spawn Player`
  (params (CurrentPlayerIndex :type Integer) (InputReceiver :type "/Game/_Main/GameMode/BP_InputReciever Object Reference"))
  (returns (Return :type Boolean))
  (bind _returnvalue (`|SpawnActorFromClass` "/Game/_Main/GameMode/BP_MainMenuCharacter.BP_MainMenuCharacter_C" (`self.GetTransform` (`local.InputReceiver`)) "Undefined" "OverrideRootScale" null (`local.CurrentPlayerIndex`) null))
  (`Controller.Possess` (`GameplayStatics.GetPlayerController` (`local.CurrentPlayerIndex`)) _returnvalue)
  (return false))

(fn `UserConstructionScript`)