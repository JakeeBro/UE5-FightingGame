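; BP_MainMenuCharacter is a main menu player character with basic movement and look controls.
; BeginPlay sets the IAC_FighterInput3D mapping context for its Index.
; Move inputs follow forward and right vectors from control-rotation yaw via FGetMovementDirection, while look and turn inputs drive controller pitch and yaw.
; Debug prints show the move-forward value every Tick and the Index on the face-down button.
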(event `self.ReceiveBeginPlay`
  (`/Game/_Main/Functions/L_CharacterMacros.Set Input Mapping Context` "/Game/_Main/Input/IAC_FighterInput3D.IAC_FighterInput3D" (`self.Index`)))

(event `self.ReceiveTick`
  (params (DeltaSeconds :type "Float (single-precision)"))
  (`KismetSystemLibrary.PrintString` (`KismetStringLibrary.Conv_DoubleToString` (`|GetInputActionValue`)) true false (struct :`G` 0.66 :`B` 1.0 :`A` 1.0) 0.0))

(event `EnhancedInput|/Game/_Main/Input/IA_MoveForward`
  (params (ActionValue :type "Float (single-precision)") (ElapsedSeconds :type "Float (single-precision)") (TriggeredSeconds :type "Float (single-precision)"))
  ;[1 1 1] Movement
  (:`Triggered`
    (`self.AddMovementInput` (`self.F_GetMovementDirection`) ActionValue)))

(event `EnhancedInput|/Game/_Main/Input/IA_Look`
  (params (ActionValue :type "Float (single-precision)") (ElapsedSeconds :type "Float (single-precision)") (TriggeredSeconds :type "Float (single-precision)"))
  ;[1 1 1] Look
  (:`Triggered`
    (`self.AddControllerPitchInput` ActionValue)))

(event `EnhancedInput|/Game/_Main/Input/IA_Turn`
  (params (ActionValue :type "Float (single-precision)") (ElapsedSeconds :type "Float (single-precision)") (TriggeredSeconds :type "Float (single-precision)"))
  ;[1 1 1] Look
  (:`Triggered`
    (`self.AddControllerYawInput` ActionValue)))

(event `EnhancedInput|/Game/_Main/Input/IA_MoveRight`
  (params (ActionValue :type "Float (single-precision)") (ElapsedSeconds :type "Float (single-precision)") (TriggeredSeconds :type "Float (single-precision)"))
  ;[1 1 1] Movement
  (:`Triggered`
    (`self.AddMovementInput` (`.Right` (`self.F_GetMovementDirection`)) ActionValue)))

(event `EnhancedInput|/Game/_Main/Input/IA_Face_Down`
  (params (ActionValue :type Boolean) (ElapsedSeconds :type "Float (single-precision)") (TriggeredSeconds :type "Float (single-precision)"))
  (:`Triggered`
    (`KismetSystemLibrary.PrintString` (`KismetStringLibrary.Conv_IntToString` (`self.Index`)))))

(fn `F_GetMovementDirection`
  (returns (Forward :type "Vector Structure") (Right :type "Vector Structure"))
  (bind _returnvalue (`KismetMathLibrary.MakeRotator` 0.0 0.0 (.yaw (`self.GetControlRotation`))))
  (return (`KismetMathLibrary.GetForwardVector` _returnvalue) (`KismetMathLibrary.GetRightVector` _returnvalue)))

(fn `UserConstructionScript`)