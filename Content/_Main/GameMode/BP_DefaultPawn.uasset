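; BP_DefaultPawn is a placeholder pawn that handles drop-in local multiplayer joining through the Join input.
; On press it creates a local player, then spawns a BP_PlayerStart at the active level's spawn point for the first inactive slot to spawn that player.
; It then spawns a fresh copy of itself at the next inactive slot's spawn point and destroys itself.
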(event `InputAction|Join`
  (params (Key :type "Key Structure"))
  (bind _bp_game_instance (`/Game/_Main/Functions/L_LogicFunctions.F_GetGameInstance`))
  (:`Pressed`
    (bind _slot_index (`/Game/_Main/GameMode/BP_GameInstance.F_FirstInactiveSlot` _bp_game_instance))
    (bind _level (`/Game/_Main/GameMode/BP_GameInstance.F_GetActiveLevel` _bp_game_instance))
    (bind _spawn_point (`/Game/_Main/Maps/BP_Level.F_GetSpawnPointByIndex` _level _slot_index))
    (`GameplayStatics.CreatePlayer` -1)
    (bind _returnvalue (`|SpawnActorFromClass` "/Game/_Main/GameMode/BP_PlayerStart.BP_PlayerStart_C" _spawn_point "AlwaysSpawn" "OverrideRootScale" null _slot_index null))
    (bind _player (`/Game/_Main/GameMode/BP_PlayerStart.F_SpawnPlayer` _returnvalue))
    (`KismetSystemLibrary.PrintString` (`KismetStringLibrary.Conv_TransformToString` (`self.GetTransform` _player)))
    (bind _slot_index_2 (`/Game/_Main/GameMode/BP_GameInstance.F_FirstInactiveSlot` _bp_game_instance))
    (bind _level_2 (`/Game/_Main/GameMode/BP_GameInstance.F_GetActiveLevel` _bp_game_instance))
    (bind _spawn_point_2 (`/Game/_Main/Maps/BP_Level.F_GetSpawnPointByIndex` _level_2 _slot_index_2))
    (`|SpawnActorFromClass` "BP_DefaultPawn_C" _spawn_point_2 "Undefined" "OverrideRootScale" null null)
    (`self.K2_DestroyActor`)))

(fn `UserConstructionScript`)