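; BP_PlayerStart is an indexed player start that spawns and possesses a main menu character for the player with the matching index.
; On BeginPlay it converts its Index into its PlayerStartTag.
; F_SpawnPlayer spawns BP_MainMenuCharacter at the start's transform regardless of collision, passes it the Index and has that player controller possess it.
; Nothing in this Blueprint calls F_SpawnPlayer, so spawning is left to external callers.
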(event `self.ReceiveBeginPlay`
  (`self.F_SetPlayerStartTagIndex`))

(fn `F_SetPlayerStartTagIndex`
  (returns (`Player Start Tag` :type Name) (Index :type Integer))
  (bind _index (`self.Index`))
  (bind _output_get (set `self.PlayerStartTag` (`KismetStringLibrary.Conv_StringToName` (`KismetStringLibrary.Conv_IntToString` _index))))
  (return _output_get _index))

(fn `F_SpawnPlayer`
  (returns (Player :type "/Game/_Main/GameMode/BP_MainMenuCharacter Object Reference"))
  (bind _returnvalue (`|SpawnActorFromClass` "/Game/_Main/GameMode/BP_MainMenuCharacter.BP_MainMenuCharacter_C" (`self.GetTransform`) "AlwaysSpawn" "OverrideRootScale" null (`self.Index`) null))
  (`Controller.Possess` (`GameplayStatics.GetPlayerController` (`self.Index`)) _returnvalue)
  (return _returnvalue))

(fn `UserConstructionScript`)