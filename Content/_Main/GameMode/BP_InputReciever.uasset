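; BP_InputReciever listens for the Start input and asks the game mode to spawn a player for its PlayerIndex.
; BeginPlay adds the IAC_MainMenu mapping context to the Enhanced Input subsystem of player controller 0, whatever the receiver's index.
; IA_Start calls SpawnPlayerMessage on the game mode with the index and itself, then prints the index.
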(event `self.ReceiveBeginPlay`
  (`EnhancedInputSubsystemInterface.AddMappingContext` (pcsubsystem `EnhancedInputLocalPlayerSubsystem` (`GameplayStatics.GetPlayerController` 0)) "/Game/_Main/Input/IAC_MainMenu.IAC_MainMenu" 0))

(event `EnhancedInput|/Game/_Main/Input/IA_Start`
  (params (ActionValue :type Boolean) (ElapsedSeconds :type "Float (single-precision)") (TriggeredSeconds :type "Float (single-precision)"))
  (:`Triggered`
    (message `/Game/_Main/GameMode/INT_GameMode.Spawn Player` (`GameplayStatics.GetGameMode`) (`self.PlayerIndex`) self)
    (`KismetSystemLibrary.PrintString` (`KismetStringLibrary.Conv_IntToString` (`self.PlayerIndex`)))))

(fn `UserConstructionScript`)