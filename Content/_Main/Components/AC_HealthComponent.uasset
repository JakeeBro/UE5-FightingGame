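; AC_HealthComponent is an actor component that tracks the owner's current health.
; On BeginPlay, a reset macro sets current health to max health.
; A modify function subtracts or adds an amount based on a damage flag and returns the new value, with no clamping or death handling.
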(event `self.ReceiveBeginPlay`
  (`self.M Reset Health`))

(fn `F_ModifyHealth`
  (params (Damage :type Boolean) (Amount :type "Float (double-precision)"))
  (returns (Health :type "Float (double-precision)"))
  (bind _currenthealth (`self.CurrentHealth`))
  (if Damage
    (bind _output_get (set `self.CurrentHealth` (- _currenthealth Amount)))
    (return _output_get)
    (else
      (bind _output_get_2 (set `self.CurrentHealth` (+ _currenthealth Amount)))
      (return _output_get_2))))